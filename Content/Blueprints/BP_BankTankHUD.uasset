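; BP_BankTankHUD is the game's HUD Blueprint, showing gun status, score and a crosshair.
; On BeginPlay it creates BP_GunStatusWidget and BP_ScoreWidget and adds both to the viewport.
; DrawHUD draws the Crosshair texture each frame at half the screen size, scaled by CrosshairSize, with no offset for the texture's own dimensions.
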(event EventDrawHUD
  (params (SizeX :type Integer) (SizeY :type Integer))
  (Class|HUD|DrawTextureSimple "/Game/HUD/crosshair.crosshair" (Math|Conversions|ToFloat(Integer) (/ SizeX 2)) (Math|Conversions|ToFloat(Integer) (/ SizeY 2)) (Variables|Default|GetCrosshairSize) false))

(event EventBeginPlay
  (bind _returnvalue (UserInterface|CreateWidget "/Game/Blueprints/BP_GunStatusWidget.BP_GunStatusWidget_C"))
  (bind _returnvalue_2 (UserInterface|CreateWidget "/Game/Blueprints/BP_ScoreWidget.BP_ScoreWidget_C"))
  (UserInterface|Viewport|AddtoViewport (Utilities|Array|MakeArray _returnvalue _returnvalue_2) 0))

(fn ConstructionScript)